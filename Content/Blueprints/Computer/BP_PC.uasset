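; BP_PC is an in-world computer whose widget screen the first-person player can point at and click.
; Each tick, a short object trace from the player camera sets whether the screen is targeted.
; The hit's collision UV is mapped to the widget's draw size to slide the WidgetInteraction component across the screen as a pointer.
; Interact simulates a one-tick left mouse click while the screen is targeted.
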(event `self.ReceiveBeginPlay`
  (set `self.InteractionStart` (`SceneComponent.RelativeLocation` (`self.WidgetInteraction`))))

(event `/Game/Blueprints/BPI_Interact.Interact`
  (params (Caller :type "Actor Object Reference"))
  (bind _widgetinteraction (`self.WidgetInteraction`))
  (if (`self.ScreenAttentive`)
    (`WidgetInteractionComponent.PressPointerKey` _widgetinteraction "LeftMouseButton")
    (`KismetSystemLibrary.DelayUntilNextTick`)
    (`WidgetInteractionComponent.ReleasePointerKey` _widgetinteraction "LeftMouseButton")))

(event `self.ReceiveTick`
  (params (DeltaSeconds :type "Float (single-precision)"))
  (bind _returnvalue (`WidgetComponent.GetCurrentDrawSize` (`self.Widget`)))
  (bind (_x _y) (`KismetMathLibrary.BreakVector2D` _returnvalue))
  (bind (_returnvalue_x _returnvalue_y) (`KismetMathLibrary.BreakVector2D` (* _returnvalue 0.5)))
  (bind _asbp_first_person_character (cast `/Game/FirstPersonContent/FirstPerson/Blueprints/BP_FirstPersonCharacter` (`GameplayStatics.GetPlayerPawn` 0)))
  (bind _firstpersoncamera (`/Game/FirstPersonContent/FirstPerson/Blueprints/BP_FirstPersonCharacter.FirstPersonCamera` _asbp_first_person_character))
  (bind _returnvalue_2 (`SceneComponent.K2_GetComponentLocation` _firstpersoncamera))
  (bind (_outhit _returnvalue_3) (`KismetSystemLibrary.LineTraceSingleForObjects` :`Start` _returnvalue_2 :`End` (+ _returnvalue_2 (* (`SceneComponent.GetForwardVector` _firstpersoncamera) 300.0)) :`ObjectTypes` (`|MakeArray` "ObjectTypeQuery7" :!type "EObjectTypeQuery Enum") :`bTraceComplex` true :`bIgnoreSelf` false))
  (if _returnvalue_3
    (set `self.ScreenAttentive` true)
    (bind (_x_2 _y_2) (`KismetMathLibrary.BreakVector2D` (`GameplayStatics.FindCollisionUV` _outhit 1)))
    (`SceneComponent.K2_SetRelativeLocation` (`self.WidgetInteraction`) (+ (`KismetMathLibrary.MakeVector` 0.0 (`KismetMathLibrary.Lerp` _x 0.0 _x_2) (`KismetMathLibrary.Lerp` _y 0.0 _y_2)) (- (`self.InteractionStart`) (`KismetMathLibrary.MakeVector` 0.0 _returnvalue_x _returnvalue_y))) false false)
    (else
      (set `self.ScreenAttentive` false))))

(fn `UserConstructionScript`)