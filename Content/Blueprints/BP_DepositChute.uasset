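; BP_DepositChute is the chute where game assets are deposited for orders tracked by the GameState.
; On BeginPlay it sets the GameState's SpawnPoint to a position offset from the Chute component.
; Its Box overlap passes any entering BP_GameAsset to ItemDeposited on the GameState.
; Its Interact event takes a BP_Lever caller and calls either FlushOrder or Deliver on the GameState, depending on the lever type.
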(event `self.ReceiveBeginPlay`
  (bind _asgame_state (cast `/Game/GameManager/GameState` (`GameplayStatics.GetGameState`)))
  (set `/Game/GameManager/GameState.SpawnPoint` (+ (`SceneComponent.K2_GetComponentLocation` (`self.Chute`)) (0.0 900.0 0.0)) _asgame_state))

(event `self.Box.OnComponentBeginOverlap`
  (params (OverlappedComponent :type "PrimitiveComponent Object Reference") (OtherActor :type "Actor Object Reference") (OtherComp :type "PrimitiveComponent Object Reference") (OtherBodyIndex :type Integer) (bFromSweep :type Boolean) (SweepResult :type "HitResult Structure (by ref)"))
  (bind _asbp_game_asset (cast `/Game/Blueprints/BP_GameAsset` OtherActor))
  (bind _asgame_state (cast `/Game/GameManager/GameState` (`GameplayStatics.GetGameState`)))
  (`/Game/GameManager/GameState.ItemDeposited` _asgame_state _asbp_game_asset))

(event `/Game/Blueprints/BPI_Interact.Interact`
  (params (Caller :type "Actor Object Reference"))
  ; Flush_Lever
  (bind _asbp_lever (cast `/Game/Blueprints/BP_Lever` Caller))
  (bind _asgame_state (cast `/Game/GameManager/GameState` (`GameplayStatics.GetGameState`)))
  (bind _levtype (`/Game/Blueprints/BP_Lever.LevType` _asbp_lever))
  (if (`|EnumEquality` _levtype "NewEnumerator1")
    (`/Game/GameManager/GameState.FlushOrder` _asgame_state)
    (elif (`|EnumEquality` _levtype "NewEnumerator2")
      (`/Game/GameManager/GameState.Deliver` _asgame_state))))

(fn `UserConstructionScript`)