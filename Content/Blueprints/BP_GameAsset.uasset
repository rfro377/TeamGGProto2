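; BP_GameAsset is a data-driven physics prop that the first-person character can pick up and carry.
; On BeginPlay or RebuildAsset, it looks up its Name in DT_GameAssets to set ID, pickup transform and physics-simulated mesh.
; Interact triggers Pickup, which grabs it with the character's PhysicsHandle and raises angular damping; Release lowers the damping.
; ShrinkMesh starts a Tick-driven scale lerp that hides the mesh when finished.
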(event `self.ReceiveBeginPlay`
  (bind _staticmesh (`self.StaticMesh`))
  (if (!= (`self.name`) "test")
    ; Build from DataTable
    (bind _returnvalue (`|GetDataTableRow` "/Game/GameManager/DT_GameAssets.DT_GameAssets" (`self.name`) :!label _label)
      (:`then`
        (bind (_asset_id _pickup_transform _assettype _gamegenre _static_mesh) (break `/Game/GameManager/Struct_GameAsset` _returnvalue))
        (set `self.Asset_ID` _asset_id)
        (set `self.PickupTransform` _pickup_transform)
        (`StaticMeshComponent.SetStaticMesh` _staticmesh _static_mesh)
        (`PrimitiveComponent.SetSimulatePhysics` _staticmesh true)
        (`PrimitiveComponent.SetCollisionResponseToChannel` _staticmesh "ECC_GameTraceChannel1" "ECR_Block")))))

(event `RebuildAsset`
  (params (UpdateName :type Name))
  ; Build from DataTable
  (set `self.name` UpdateName)
  (goto _label))

(event `self.ReceiveTick`
  (params (DeltaSeconds :type "Float (single-precision)"))
  (bind _staticmesh (`self.StaticMesh`))
  (bind _shrinkalpha (`self.ShrinkAlpha`))
  ; Tick
  (`|ExecutionSequence`
    (:`then_0`
      (if (`self.isShrinking`)
        (`SceneComponent.SetWorldScale3D` _staticmesh (`KismetMathLibrary.VLerp` (`SceneComponent.K2_GetComponentScale` _staticmesh) (0.1 0.1 0.1) (/ _shrinkalpha (`self.LerpSpeed`))))
        (bind _output_get (set `self.ShrinkAlpha` (`KismetMathLibrary.FClamp` (/ (+ _shrinkalpha DeltaSeconds) (`self.LerpSpeed`)))))
        (if (== _output_get 1.0)
          (`SceneComponent.SetVisibility` (`self.StaticMesh`) false false))))))

(event `Pickup`
  (params (Caller :type "Actor Object Reference"))
  ; Base Pickup Code
  (bind _asbp_first_person_character (cast `/Game/FirstPersonContent/FirstPerson/Blueprints/BP_FirstPersonCharacter` Caller))
  (set `/Game/FirstPersonContent/FirstPerson/Blueprints/BP_FirstPersonCharacter.isCarrying?` true _asbp_first_person_character)
  (set `/Game/FirstPersonContent/FirstPerson/Blueprints/BP_FirstPersonCharacter.CarriedActor` self _asbp_first_person_character)
  (set `self.isPickedUp?` true)
  (`PrimitiveComponent.SetAngularDamping` (`self.StaticMesh`) 100.0)
  (bind (_lasthit_bblockinghit _lasthit_binitialoverlap _lasthit_time _lasthit_distance _lasthit_location _lasthit_impactpoint _lasthit_normal _lasthit_impactnormal _lasthit_physmat _lasthit_hitactor _lasthit_hitcomponent) (`GameplayStatics.BreakHitResult` (`/Game/FirstPersonContent/FirstPerson/Blueprints/BP_FirstPersonCharacter.LastHit` _asbp_first_person_character)))
  (`PhysicsHandleComponent.GrabComponentAtLocation` (`/Game/FirstPersonContent/FirstPerson/Blueprints/BP_FirstPersonCharacter.PhysicsHandle` _asbp_first_person_character) _lasthit_hitcomponent "None" _lasthit_location))

(event `/Game/Blueprints/BPI_Interact.Interact`
  (params (Caller :type "Actor Object Reference"))
  ; PickupCall
  (`self.Pickup` Caller))

(event `Release`
  ; Release Event
  (`PrimitiveComponent.SetAngularDamping` (`self.StaticMesh`) 1.0))

(event `ShrinkMesh`
  ; ShrinkMesh
  (set `self.isShrinking` true)
  (set `self.ShrinkAlpha` 0.0))

(fn `UserConstructionScript`)