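; BP_Trolley is an interactable trolley that the first-person character grabs and pushes around.
; On Interact, it snaps its static mesh to floor level ahead of the calling character and yaws it to align with the character's facing.
; It then attaches the actor to the character keeping world position and rotation, and lowers walk speed and camera speed multiplier.
; The Blueprint has no release or detach logic.
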(event `/Game/Blueprints/BPI_Interact.Interact`
  (params (Caller :type "Actor Object Reference"))
  (bind _staticmesh (`self.StaticMesh`))
  (bind _asbp_first_person_character (cast `/Game/FirstPersonContent/FirstPerson/Blueprints/BP_FirstPersonCharacter` Caller))
  (bind _capsulecomponent (`Character.CapsuleComponent` _asbp_first_person_character))
  (bind (_returnvalue_x _returnvalue_y) (`KismetMathLibrary.BreakVector` (`SceneComponent.GetForwardVector` _capsulecomponent)))
  (bind (_returnvalue_location _returnvalue_rotation) (`KismetMathLibrary.BreakTransform` (`self.GetTransform` _asbp_first_person_character)))
  (`SceneComponent.K2_SetWorldLocation` _staticmesh (+ (+ (* (`KismetMathLibrary.Normal` (`KismetMathLibrary.MakeVector` _returnvalue_x _returnvalue_y)) 300.0) (`KismetMathLibrary.MakeVector` 0.0 0.0 (* (`CapsuleComponent.GetScaledCapsuleHalfHeight` _capsulecomponent) -1.0))) _returnvalue_location) false false)
  (bind (_returnvalue_roll _returnvalue_pitch _returnvalue_yaw) (`KismetMathLibrary.BreakRotator` (`KismetMathLibrary.MakeRotFromX` (`KismetMathLibrary.Conv_RotatorToVector` _returnvalue_rotation))))
  (`SceneComponent.K2_SetWorldRotation` _staticmesh (`KismetMathLibrary.MakeRotator` 0.0 0.0 (+ _returnvalue_yaw -90.0)) false false)
  (`self.K2_AttachToActor` _asbp_first_person_character "None" "KeepWorld" "KeepWorld" "KeepRelative")
  (set `CharacterMovementComponent.MaxWalkSpeed` 250.0 (`Character.CharacterMovement` _asbp_first_person_character))
  (set `/Game/FirstPersonContent/FirstPerson/Blueprints/BP_FirstPersonCharacter.CameraSpeedMult` 0.5 _asbp_first_person_character))

(fn `UserConstructionScript`)