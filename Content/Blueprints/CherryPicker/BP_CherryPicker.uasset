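; BP_CherryPicker is an interactable lift whose platform the first-person character can raise and lower.
; Interact toggles movement and flips the direction whenever it starts, so interacting mid-travel halts the platform and the next use reverses it.
; While running, Tick eases the platform's relative location toward the raised or base position with VInterpTo, stopping once within a tolerance of the target.
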(event `self.ReceiveTick`
  (params (DeltaSeconds :type "Float (single-precision)"))
  (bind _platform (`self.Platform`))
  (bind _relativelocation (`SceneComponent.RelativeLocation` (`self.Platform`)))
  (bind _returnvalue (`KismetMathLibrary.VInterpTo` _relativelocation (0.0 0.0 0.0) DeltaSeconds 0.6))
  (bind _returnvalue_2 (`KismetMathLibrary.VInterpTo` _relativelocation (0.0 0.0 200.0) DeltaSeconds 0.6))
  (if (`self.isRun`)
    (if (`self.Extended?`)
      (`SceneComponent.K2_SetRelativeLocation` _platform _returnvalue_2 false false)
      (if (== _returnvalue_2 (0.0 0.0 200.0) :`ErrorTolerance` 20.0)
        (set `self.isRun` false :!label _label))
      (else
        (`SceneComponent.K2_SetRelativeLocation` _platform _returnvalue false false)
        (if (== _returnvalue (0.0 0.0 0.0) :`ErrorTolerance` 20.0)
          (goto _label))))))

(event `/Game/Blueprints/BPI_Interact.Interact`
  (params (Caller :type "Actor Object Reference"))
  (cast `/Game/FirstPersonContent/FirstPerson/Blueprints/BP_FirstPersonCharacter` Caller)
  (bind _output_get (set `self.isRun` (not (`self.isRun`))))
  (if _output_get
    (set `self.Extended?` (not (`self.Extended?`)))))

(fn `UserConstructionScript`)